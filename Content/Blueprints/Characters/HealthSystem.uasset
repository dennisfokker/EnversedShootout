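; Player-state health component that treats a character's limbs as ordered health stages, lost one at a time.
; After a short BeginPlay delay, the server maps the pawn's BP_LimbComponents by their order index.
; OnLimbHit damages the current stage's limb; a depleted limb triggers its loss and advances the index, with death only printed after the last.
; ResetLimbsAndHealth restores the character's colors, limb hit points and collision, and rewinds the stage.
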(event `self.ReceiveBeginPlay`
  ;[0.06301 1 0] Event BeginPlay
  ;;[1 1 1] Add all Limbs to the HeatlhSystem
  ;;;[1 1 1] Delay 1 frame because character initializes too slowly
  (`KismetSystemLibrary.Delay` 0.1)
  (if (`Actor.HasAuthority` (`self.GetOwner`))
    (bind _playerpawn (`self.GetPlayerPawn`))
    (`/Engine/EditorBlueprintResources/StandardMacros.IsValid` _playerpawn
      (:`Is Valid`
        (bind _returnvalue (`Actor.K2_GetComponentsByClass` _playerpawn "/Game/Blueprints/Characters/BP_LimbComponent.BP_LimbComponent_C"))
        (if (`KismetArrayLibrary.Array_IsValidIndex` _returnvalue)
          (for _array_element _returnvalue
            (`BlueprintMapLibrary.Map_Add` (`self.LimbOrder`) (`/Game/Blueprints/Characters/BP_LimbComponent.OrderInHealthSystem` _array_element) _array_element)))))))

(event `OnLimbHit`
  (bind (_value _returnvalue) (`BlueprintMapLibrary.Map_Find` (`self.LimbOrder`) (`self.CurrentStageIndex`)))
  (bind _returnvalue_2 (- (`/Game/Blueprints/Characters/BP_LimbComponent.HitPoints` _value) 1))
  ;[1 0 0.855] Event OnHit
  ;;[1 1 1] Remove Limb health and run OnLimbLoss if needed
  (if (`self.DoesComponentHaveAuthority`)
    (if _returnvalue
      (set `/Game/Blueprints/Characters/BP_LimbComponent.HitPoints` _returnvalue_2 _value)
      (if (<= _returnvalue_2 0)
        (bind _playerstate (`self.GetPlayerState`))
        (`self.OnLimbLoss` _playerstate)))))

(fn `GetCollisions`
  (params (Index :type Integer))
  (returns (Collisions :type "Array of PrimitiveComponent Object Reference"))
  (return (`/Game/Blueprints/Characters/BP_LimbComponent.Collisions` (`BlueprintMapLibrary.Map_Find` (`self.LimbOrder`) Index))))

(fn `GetMeshes`
  (params (Index :type Integer))
  (returns (Meshes :type "Array of StaticMeshComponent Object Reference"))
  (return (`/Game/Blueprints/Characters/BP_LimbComponent.Meshes` (`BlueprintMapLibrary.Map_Find` (`self.LimbOrder`) Index))))

(fn `GetPlayerPawn`
  (returns (PlayerPawn :type "Pawn Object Reference"))
  (locals (ChosenPawn :type "Pawn Object Reference"))
  (bind _returnvalue (`GameplayStatics.GetGameState`))
  (`/Engine/EditorBlueprintResources/StandardMacros.IsValid` _returnvalue
    (:`Is Valid`
      (for (_array_element _array_index) (`GameStateBase.PlayerArray` _returnvalue)
        (if (== _array_element (`self.GetOwner`))
          (set `local.ChosenPawn` (`Controller.K2_GetPawn` (`GameplayStatics.GetPlayerController` _array_index)))
          (break)))
      (return (`local.ChosenPawn`)))))

(fn `GetPlayerState`
  (returns (PlayerState :type "/Game/Blueprints/ModesAndStates/ScorePlayerState Object Reference"))
  (bind _returnvalue (`GameplayStatics.GetGameState`))
  (`/Engine/EditorBlueprintResources/StandardMacros.IsValid` _returnvalue
    (:`Is Valid`
      (for (_array_element _array_index) (`GameStateBase.PlayerArray` _returnvalue)
        (if (== _array_element (`self.GetOwner`))
          (bind _asscore_player_state (cast `/Game/Blueprints/ModesAndStates/ScorePlayerState` (`Controller.PlayerState` (`GameplayStatics.GetPlayerController` _array_index))))
          (return _asscore_player_state))))))

(fn `OnAllLimbsLost`
  (`KismetSystemLibrary.PrintString` "Player Died")
  (return))

(fn `OnLimbLoss`
  (params (TargetPlayer :type "/Game/Blueprints/ModesAndStates/ScorePlayerState Object Reference"))
  (locals (bAllLimbsLost :type Boolean :default true))
  ;[1 1 1] Check if this was the last Limb
  (`/Game/Blueprints/Characters/BP_LimbComponent.OnLimbLoss` (`BlueprintMapLibrary.Map_Find` (`self.LimbOrder`) (`self.CurrentStageIndex`)) TargetPlayer)
  (`/Engine/EditorBlueprintResources/StandardMacros.IncrementInt` (`self.CurrentStageIndex`)
    (:`  `
      (if (not (`.ReturnValue` (`BlueprintMapLibrary.Map_Find` (`self.LimbOrder`) (`self.CurrentStageIndex`))))
        (`self.OnAllLimbsLost`)
        (return)))))

(fn `ResetLimbsAndHealth`
  (locals (PlayerCharacter :type "/Game/Blueprints/Characters/FirstPersonCharacter Object Reference"))
  (bind _playercharacter (`local.PlayerCharacter`))
  ;[1 1 1] Get character
  (bind _outactors (`GameplayStatics.GetAllActorsOfClass` "/Game/Blueprints/Characters/FirstPersonCharacter.FirstPersonCharacter_C"))
  (for _array_element _outactors
    (if (== (`Pawn.PlayerState` _array_element) (`self.GetOwner`))
      (bind _output_get (set `local.PlayerCharacter` _array_element))
      (break)))
  (`/Engine/EditorBlueprintResources/StandardMacros.IsValid` _output_get
    (:`Is Valid`
      ;[1 1 1] Reset all limbs (visual, variables and collision)
      (`/Game/Blueprints/Characters/FirstPersonCharacter.DrawPlayerInColor` _playercharacter)
      (for _array_element_2 (`Actor.K2_GetComponentsByClass` _playercharacter "/Game/Blueprints/Characters/BP_LimbComponent.BP_LimbComponent_C")
        (set `/Game/Blueprints/Characters/BP_LimbComponent.HitPoints` 1 _array_element_2)
        (for _array_element_3 (`/Game/Blueprints/Characters/BP_LimbComponent.Collisions` _array_element_2)
          (`PrimitiveComponent.SetCollisionEnabled` _array_element_3 "QueryOnly")))
      (set `self.CurrentStageIndex` 0)
      (return))
    (:`Is Not Valid`
      (return))))