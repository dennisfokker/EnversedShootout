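; BP_LimbComponent is a character limb component that changes the limb's look and removes its collision when the limb is lost.
; On BeginPlay it gathers all descendant components tagged "Limb", storing static meshes in Meshes and other primitive components in Collisions.
; OnLimbLoss applies BaseMaterial to the first material slot of each mesh and disables collision only on the components in Collisions.
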(event `OnLimbLoss`
  ;[1 0 0.855] Event OnHit
  ;;[1 1 1] Remove Collision of Limb and Change color
  (for _array_element (`self.Meshes`)
    (`/Engine/EditorBlueprintResources/StandardMacros.IsValid` _array_element
      (:`Is Valid`
        (`PrimitiveComponent.SetMaterial` _array_element 0 "/Game/Assets/Materials/BaseMaterial.BaseMaterial"))))
  (for _array_element_2 (`self.Collisions`)
    (`/Engine/EditorBlueprintResources/StandardMacros.IsValid` _array_element_2
      (:`Is Valid`
        (`PrimitiveComponent.SetCollisionEnabled` _array_element_2 "NoCollision")))))

(event `self.ReceiveBeginPlay`
  ;[0.06301 1 0] Event BeginPlay
  ;;[1 1 1] Add meshes and collisions to this component
  (for _array_element (`self.GetChildrenComponents` true)
    (if (`self.ComponentHasTag` _array_element "Limb")
      (bind _asstatic_mesh_component (cast `StaticMeshComponent` _array_element)
        (:`then`
          (`KismetArrayLibrary.Array_Add` (`self.Meshes`) _asstatic_mesh_component))
        (:`CastFailed`
          (bind _asprimitive_component (cast `PrimitiveComponent` _array_element))
          (`KismetArrayLibrary.Array_Add` (`self.Collisions`) _asprimitive_component)))))
  (if true
    _))