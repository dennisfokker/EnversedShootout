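; BouncyPad is an environment pad that deflects projectiles toward the head of the shooter's opponent.
; On overlap, the server finds the first entry in its Characters array that is not the projectile's instigator and computes a look-at rotation to that head.
; A multicast then rotates the projectile and reapplies its original local-space velocity, so it keeps its speed along the new heading.
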(event `self.BaseMesh.OnComponentBeginOverlap`
  (params (OverlappedComponent :type "PrimitiveComponent Object Reference") (OtherActor :type "Actor Object Reference") (OtherComp :type "PrimitiveComponent Object Reference") (OtherBodyIndex :type Integer) (bFromSweep :type Boolean) (SweepResult :type "HitResult Structure (by ref)"))
  ;[1 0 0.9013] Event Hit
  ;;[1 1 1] Rotate projectile towards other player.
  (`/Engine/EditorBlueprintResources/ActorMacros.Switch Has Authority`
    (:`Authority`
      (bind _asbase_projectile (cast `/Game/Blueprints/Weapons/Projectiles/BaseProjectile` OtherActor))
      (bind _asfirst_person_character (cast `/Game/Blueprints/Characters/FirstPersonCharacter` (`self.GetInstigator` _asbase_projectile)))
      (bind _opponenthead (`self.GetHeadOfOpponent` _asfirst_person_character))
      (bind _output_get (set `self.LocalVelocity` (`KismetMathLibrary.LessLess_VectorRotator` (`MovementComponent.Velocity` (`/Game/Blueprints/Weapons/Projectiles/BaseProjectile.Projectile` _asbase_projectile)) (`self.K2_GetActorRotation` _asbase_projectile))))
      (`self.Multicast_ChangeDirection` (`KismetMathLibrary.FindLookAtRotation` (`self.K2_GetActorLocation` _asbase_projectile) (`SceneComponent.K2_GetComponentLocation` _opponenthead)) _output_get _asbase_projectile))))

(event `Multicast_ChangeDirection`
  (params (Rotator :type "Rotator Structure") (Velocity :type "Vector Structure") (BaseProjectile :type "/Game/Blueprints/Weapons/Projectiles/BaseProjectile Object Reference"))
  (`self.K2_SetActorRotation` BaseProjectile Rotator false)
  (`ProjectileMovementComponent.SetVelocityInLocalSpace` (`/Game/Blueprints/Weapons/Projectiles/BaseProjectile.Projectile` BaseProjectile) Velocity))

(fn `GetHeadOfOpponent`
  (params (Player :type "/Game/Blueprints/Characters/FirstPersonCharacter Object Reference"))
  (returns (OpponentHead :type "StaticMeshComponent Object Reference"))
  (for _array_element (`self.Characters`)
    (if (!= _array_element Player)
      (return (`/Game/Blueprints/Characters/FirstPersonCharacter.Head` _array_element)))))

(fn `UserConstructionScript`)