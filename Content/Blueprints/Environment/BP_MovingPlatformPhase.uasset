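; Moving platform variant that steps between start and end locations in discrete phases, driven by keyboard input on the authority.
; The authority enables input from player 0, and bracket or comma/period keys raise or lower CurrentPhase within zero to TotalPhases.
; An overridden GetNextTransform interpolates the phase's position, which a multicast event applies as a swept move.
; Reset returns the platform to phase zero.
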(event `self.ReceiveBeginPlay`
  ;[0.06301 1 0] Allow input consumption
  (`/Engine/EditorBlueprintResources/ActorMacros.Switch Has Authority`
    (:`Authority`
      (`self.EnableInput` (`GameplayStatics.GetPlayerController` 0)))))

(event `Key|LeftBracket` :consume false :overrideparent false
  (params (Key :type "Key Structure"))
  ;[1 1 0] Go to next/previous phase
  (:`Pressed`
    (`/Engine/EditorBlueprintResources/ActorMacros.Switch Has Authority` :!label _label
      (:`Authority`
        (bind _successful (`self.IncrementPhase`))
        (if _successful
          (bind _newtransform (`self.GetNextTransform` 0.0 :!label _label_2))
          (`self.MultiEvent_UpdateLocation` (.location _newtransform)))))))

(event `Key|Period` :consume false :overrideparent false
  (params (Key :type "Key Structure"))
  ;[1 1 0] Go to next/previous phase
  (:`Pressed`
    (goto _label)))

(event `Key|RightBracket` :consume false :overrideparent false
  (params (Key :type "Key Structure"))
  ;[1 1 0] Go to next/previous phase
  (:`Pressed`
    (`/Engine/EditorBlueprintResources/ActorMacros.Switch Has Authority` :!label _label_3
      (:`Authority`
        (bind _successful (`self.DecrementPhase`))
        (if _successful
          (goto _label_2))))))

(event `Key|Comma` :consume false :overrideparent false
  (params (Key :type "Key Structure"))
  ;[1 1 0] Go to next/previous phase
  (:`Pressed`
    (goto _label_3)))

(event `MultiEvent_UpdateLocation`
  (params (NewLocation :type "Vector Structure"))
  ;[1 1 0] Go to next/previous phase
  (`self.K2_SetActorLocation` NewLocation true))

(event `self.Reset`
  (set `self.CurrentPhase` 0)
  (bind _newtransform (`self.GetNextTransform` 0.0))
  (`self.MultiEvent_UpdateLocation` (.location _newtransform)))

(fn `DecrementPhase`
  (returns (Successful :type Boolean))
  ;[1 1 1] Check if already at last phase
  (if (<= (`self.CurrentPhase`) 0)
    (return false)
    (else
      ;[1 1 1] If can increment, increment
      (`/Engine/EditorBlueprintResources/StandardMacros.DecrementInt` (`self.CurrentPhase`)
        (:`  `
          (return true))))))

(fn `GetNextTransform`
  (params (DeltaSeconds :type "Float (double-precision)"))
  (returns (NewTransform :type "Transform Structure"))
  (bind _startlocation_location (`KismetMathLibrary.BreakTransform` (`self.StartLocation`)))
  (bind _endlocation_location (`KismetMathLibrary.BreakTransform` (`self.EndLocation`)))
  (bind _startlocation_location_2 (`KismetMathLibrary.BreakTransform` (`self.StartLocation`)))
  (`parent.GetNextTransform` DeltaSeconds)
  (return (`KismetMathLibrary.Conv_VectorToTransform` (- _startlocation_location_2 (* (/ (- _startlocation_location _endlocation_location) (`self.TotalPhases`)) (`self.CurrentPhase`))))))

(fn `IncrementPhase`
  (returns (Successful :type Boolean))
  ;[1 1 1] Check if already at last phase
  (if (>= (`self.CurrentPhase`) (`self.TotalPhases`))
    (return false)
    (else
      ;[1 1 1] If can increment, increment
      (`/Engine/EditorBlueprintResources/StandardMacros.IncrementInt` (`self.CurrentPhase`)
        (:`  `
          (return true))))))

(fn `UserConstructionScript`)