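; MovingPlatform is an actor that travels in a straight line until it hits another moving platform.
; On Tick, the authority side calls a server event that, while IsMoving is set, applies a swept world offset from MoveSpeed, its multiplier and delta time.
; A Collision component hit with an actor of the same class calls a second server event that clears IsMoving, with no logic here to restart it.
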(event `self.ReceiveTick`
  (params (DeltaSeconds :type "Float (single-precision)"))
  (`/Engine/EditorBlueprintResources/ActorMacros.Switch Has Authority`
    (:`Authority`
      (`self.Server_Event_MovePlatform` DeltaSeconds))))

(event `Server_Event_MovePlatform`
  (params (DeltaSeconds :type "Float (double-precision)"))
  (if (`self.IsMoving`)
    (`self.K2_AddActorWorldOffset` (* (* (`self.MoveSpeed`) (`self.MoveSpeedMultiplier`)) DeltaSeconds) true)))

(event `self.Collision.OnComponentHit`
  (params (HitComponent :type "PrimitiveComponent Object Reference") (OtherActor :type "Actor Object Reference") (OtherComp :type "PrimitiveComponent Object Reference") (NormalImpulse :type "Vector Structure") (Hit :type "HitResult Structure (by ref)"))
  (if (== (`GameplayStatics.GetObjectClass` OtherActor) "MovingPlatform_C")
    (`self.Server_Event_StopMoving`)))

(event `Server_Event_StopMoving`
  (set `self.IsMoving` false))

(fn `UserConstructionScript`)