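; InformationLabel is a text label actor that displays round status prompts such as waiting, countdown, shoot and hold.
; BeginPlay and OnWaiting show the waiting message, while OnCountdown steps timed prompts up to "Shoot!" and then clears the text.
; OnShooting jumps straight to "Shoot!" if the label still shows a countdown prompt, keeping it in sync, and OnCleanup shows "Hold!".
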(event `OnWaiting`
  (`TextRenderComponent.K2_SetText` (`self.TextRender`) (`KismetTextLibrary.Conv_StringToText` "Waiting...") :!label _label))

(event `self.ReceiveBeginPlay`
  (goto _label))

(event `OnCountdown`
  (`TextRenderComponent.K2_SetText` (`self.TextRender`) (`KismetTextLibrary.Conv_StringToText` "Get ready..."))
  (`KismetSystemLibrary.Delay` 2.0)
  (`TextRenderComponent.K2_SetText` (`self.TextRender`) (`KismetTextLibrary.Conv_StringToText` "Set..."))
  (`KismetSystemLibrary.Delay` 2.0)
  (`TextRenderComponent.K2_SetText` (`self.TextRender`) (`KismetTextLibrary.Conv_StringToText` "Shoot!") :!label _label_2)
  (`KismetSystemLibrary.Delay` 1.0)
  (`TextRenderComponent.K2_SetText` (`self.TextRender`) (`KismetTextLibrary.Conv_StringToText` "")))

(event `OnShooting`
  (bind _text (`TextRenderComponent.Text` (`self.TextRender`)))
  ;[1 1 1] Check if message doesn't inform shooting, otherwise quickly update it to stay in sync
  (if (or (`KismetTextLibrary.EqualEqual_TextText` (`KismetTextLibrary.Conv_StringToText` "Get ready...") _text) (== _text (`KismetTextLibrary.Conv_StringToText` "Set...")))
    (goto _label_2)))

(event `OnCleanup`
  (`TextRenderComponent.K2_SetText` (`self.TextRender`) (`KismetTextLibrary.Conv_StringToText` "Hold!")))

(fn `UserConstructionScript`)