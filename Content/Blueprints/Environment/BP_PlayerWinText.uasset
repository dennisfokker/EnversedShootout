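; BP_PlayerWinText is a world actor that announces which player color has won, using two text render components.
; Each Tick, while the root component is visible, it joins "Player", the PlayerWonColor string and "wins." and writes the result to both components.
; The file only reads PlayerWonColor and the visibility state and never sets either.
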(event `self.ReceiveTick`
  (params (DeltaSeconds :type "Float (single-precision)"))
  (bind _returnvalue (`KismetTextLibrary.Conv_StringToText` (`self.BuiltText`)))
  (if (`SceneComponent.IsVisible` (`self.DefaultSceneRoot`))
    (set `self.BuiltText` (`KismetStringLibrary.Concat_StrStr` "Player " (`KismetStringLibrary.Concat_StrStr` (`self.PlayerWonColor`) " wins.")))
    (`|ExecutionSequence`
      (:`then_0`
        (`TextRenderComponent.K2_SetText` (`self.TextRender1`) _returnvalue))
      (:`then_1`
        (`TextRenderComponent.K2_SetText` (`self.TextRender`) _returnvalue)))))

(fn `UserConstructionScript`)