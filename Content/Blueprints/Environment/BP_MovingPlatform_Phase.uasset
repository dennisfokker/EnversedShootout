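; Networked moving platform that steps between a start and end location in evenly spaced phases.
; On the authority, it enables input for player controller 0, and the Period and Comma keys step the phase forward or back within its limits.
; Each successful step interpolates the phase's location and passes it to MultiEvent_UpdateLocation, which moves the actor there with a sweep.
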(event `self.ReceiveBeginPlay`
  ;[0.06301 1 0] Allow input consumption
  (`/Engine/EditorBlueprintResources/ActorMacros.Switch Has Authority`
    (:`Authority`
      (`self.EnableInput` (`GameplayStatics.GetPlayerController` 0)))))

(event `Key|Period` :consume false :overrideparent false
  (params (Key :type "Key Structure"))
  ;[1 1 0] Go to next/previous phase
  (:`Pressed`
    (`/Engine/EditorBlueprintResources/ActorMacros.Switch Has Authority`
      (:`Authority`
        (bind _successful (`self.IncrementPhase`))
        (if _successful
          (bind _newlocation (`self.GetPhaseLocation`))
          (`self.MultiEvent_UpdateLocation` _newlocation))))))

(event `Key|Comma` :consume false :overrideparent false
  (params (Key :type "Key Structure"))
  ;[1 1 0] Go to next/previous phase
  (:`Pressed`
    (`/Engine/EditorBlueprintResources/ActorMacros.Switch Has Authority`
      (:`Authority`
        (bind _successful (`self.DecrementPhase`))
        (if _successful
          (bind _newlocation (`self.GetPhaseLocation`))
          (`self.MultiEvent_UpdateLocation` _newlocation))))))

(event `MultiEvent_UpdateLocation`
  (params (NewLocation :type "Vector Structure"))
  ;[1 1 0] Go to next/previous phase
  (`self.K2_SetActorLocation` NewLocation true))

(fn `DecrementPhase`
  (returns (Successful :type Boolean))
  ;[1 1 1] Check if already at last phase
  (if (<= (`self.CurrentPhase`) 0)
    (return false)
    (else
      ;[1 1 1] If can increment, increment
      (`/Engine/EditorBlueprintResources/StandardMacros.DecrementInt` (`self.CurrentPhase`)
        (:`  `
          (return true))))))

(fn `GetPhaseLocation`
  (returns (NewLocation :type "Vector Structure"))
  (return (- (`self.StartLocation`) (* (/ (- (`self.StartLocation`) (`self.EndLocation`)) (`self.TotalPhases`)) (`self.CurrentPhase`)))))

(fn `IncrementPhase`
  (returns (Successful :type Boolean))
  ;[1 1 1] Check if already at last phase
  (if (>= (`self.CurrentPhase`) (`self.TotalPhases`))
    (return false)
    (else
      ;[1 1 1] If can increment, increment
      (`/Engine/EditorBlueprintResources/StandardMacros.IncrementInt` (`self.CurrentPhase`)
        (:`  `
          (return true))))))

(fn `UserConstructionScript`)