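; Base Blueprint for a moving platform that holds start and end transforms.
; GetNextTransform is an empty stub, so the base defines no motion of its own.
; SetDistance replaces the start transform's Y with the given distance, signed by the lesser of the start and end Y, then calls Reset.
; Reset moves the actor to the start transform with a sweep and no teleport.
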(fn `GetNextTransform`
  (params (DeltaSeconds :type "Float (double-precision)"))
  (returns (NewTransform :type "Transform Structure"))
  (return))

(fn `Reset`
  (`self.K2_SetActorTransform` (`self.StartLocation`) true)
  (return))

(fn `SetDistance`
  (params (Distance :type "Float (double-precision)"))
  (bind _startlocation (`self.StartLocation`))
  (set `self.StartLocation` (`KismetMathLibrary.MakeTransform` (`KismetMathLibrary.MakeVector` (.x (.location _startlocation)) (* Distance (`KismetMathLibrary.SignOfFloat` (`KismetMathLibrary.FMin` (.y (.location _startlocation)) (.y (.location (`self.EndLocation`)))))) (.z (.location _startlocation))) (.rotation _startlocation) (.scale _startlocation)))
  (`self.Reset`))

(fn `UserConstructionScript`)