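; A shootable start target that begins the game once both players have hit it.
; Each overlapping projectile marks its shooter's player color as ready in a map, spawns an explosion and is destroyed on the server.
; When no map value remains false, a server-named event enables bullet increase on the FirstPersonGameMode and drops the target's root below its current position.
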(event `self.ReceiveActorBeginOverlap`
  (params (OtherActor :type "Actor Object Reference"))
  (bind _ready (`self.ready`))
  ;[1 1 1] Start the game if both player have shot this target
  (bind _asbase_projectile (cast `/Game/Blueprints/Weapons/Projectiles/BaseProjectile` OtherActor))
  (bind _asscore_player_state (cast `/Game/Blueprints/ModesAndStates/ScorePlayerState` (`Pawn.PlayerState` (`self.GetInstigator` _asbase_projectile))))
  (`BlueprintMapLibrary.Map_Add` _ready (`/Game/Blueprints/ModesAndStates/ScorePlayerState.Color` _asscore_player_state) true)
  (bind _values (`BlueprintMapLibrary.Map_Values` _ready))
  (if (not (`KismetArrayLibrary.Array_Contains` _values))
    (`self.Server_EnableBulletIncrease`))
  (`self.BulletExplosion` (`self.K2_GetActorLocation` _asbase_projectile))
  (`/Game/Blueprints/Weapons/Projectiles/BaseProjectile.DestroyOnServer` _asbase_projectile))

(event `BulletExplosion`
  (params (Location :type "Vector Structure"))
  ;[1 1 1] Bullet Explosion Event
  (`GameplayStatics.SpawnEmitterAtLocation` "/Game/External/StarterContent/Particles/P_Explosion.P_Explosion" Location (struct) (3.0 3.0 3.0)))

(event `Server_EnableBulletIncrease`
  ;[1 1 1] Start the game
  (bind _asfirst_person_game_mode (cast `/Game/Blueprints/ModesAndStates/FirstPersonGameMode` (`GameplayStatics.GetGameMode`)))
  (set `/Game/Blueprints/ModesAndStates/FirstPersonGameMode.bBulletIncreaseEnabled` true _asfirst_person_game_mode)
  (`SceneComponent.K2_SetWorldLocation` (`self.DefaultSceneRoot`) (- (`SceneComponent.K2_GetComponentLocation` (`self.DefaultSceneRoot`)) (0.0 0.0 300.0)) false false))

(fn `UserConstructionScript`)