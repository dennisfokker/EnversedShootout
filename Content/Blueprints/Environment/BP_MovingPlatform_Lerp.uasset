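; Moving platform actor that travels one way from a start transform to an end transform over a set duration.
; While IsMoving is true, Tick applies the result of GetNextTransform with a swept SetActorTransform.
; GetNextTransform lerps on elapsed time over duration, then advances the clamped time and clears IsMoving near the end.
; The lerp precedes the time update and the stop check looks a frame ahead, so motion can stop short of the end.
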(event `self.ReceiveTick`
  (params (DeltaSeconds :type "Float (single-precision)"))
  ;[1 0.305 0] Tick
  (if (`self.IsMoving`)
    (bind _newtransform (`self.GetNextTransform` DeltaSeconds))
    (`self.K2_SetActorTransform` _newtransform true)))

(fn `GetNextTransform`
  (params (DeltaSeconds :type "Float (double-precision)"))
  (returns (NewTransform :type "Transform Structure"))
  (locals (NewLerpedTransform :type "Transform Structure"))
  (bind _moveduration (`self.MoveDuration`))
  (bind _returnvalue (+ (`self.PassedTime`) DeltaSeconds))
  (bind _returnvalue_2 (>= _returnvalue _moveduration))
  ;[1 1 1] Calculate new lerped transform
  (set `local.NewLerpedTransform` (`KismetMathLibrary.TLerp` (`self.StartLocation`) (`self.EndLocation`) (/ (`self.PassedTime`) (`self.MoveDuration`))))
  ;[1 1 1] Update passed time
  (set `self.PassedTime` (select `bool` _returnvalue_2 :`false` _returnvalue :`true` _moveduration))
  ;[1 1 1] Update whether or not to move
  (if _returnvalue_2
    (set `self.IsMoving` false))
  (return (`local.NewLerpedTransform`)))

(fn `UserConstructionScript`)