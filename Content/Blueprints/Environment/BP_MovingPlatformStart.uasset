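; BP_MovingPlatformStart is a placed marker that spawns a moving platform at its own transform when play begins.
; It finds its destination by scanning all BP_MovingPlatformEnd actors for the first one with a matching ID.
; The spawned BP_MovingPlatform receives this actor's transform as its start location and the matched end marker's transform as its end location.
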(event `self.ReceiveBeginPlay`
  (bind _returnvalue (`self.GetTransform`))
  (bind _endtransform (`self.GetCorrespondingEndTransform`))
  (`|SpawnActorFromClass` "/Game/Blueprints/Environment/BP_MovingPlatform.BP_MovingPlatform_C" _returnvalue "AlwaysSpawn" "OverrideRootScale" null _returnvalue _endtransform null))

(fn `GetCorrespondingEndTransform`
  (returns (EndTransform :type "Transform Structure"))
  (locals (FoundTransform :type "Transform Structure"))
  (bind _outactors (`GameplayStatics.GetAllActorsOfClass` "/Game/Blueprints/Environment/BP_MovingPlatformEnd.BP_MovingPlatformEnd_C"))
  (for _array_element _outactors
    ;[1 1 0] Loop body
    (if (== (`/Game/Blueprints/Environment/BP_MovingPlatformEnd.ID` _array_element) (`self.ID`))
      (set `local.FoundTransform` (`self.GetTransform` _array_element))
      (break)))
  (return (`local.FoundTransform`)))

(fn `UserConstructionScript`)