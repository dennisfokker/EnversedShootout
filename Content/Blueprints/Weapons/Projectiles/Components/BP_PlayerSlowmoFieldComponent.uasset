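; Player component that slows other players' projectiles as they near its owning pawn, creating a slow-motion field.
; Every tick it stores the signed Y-axis distance to another FirstPersonCharacter, then scans all BaseProjectile actors.
; Projectiles passing a one-sided Y threshold, set as a fraction of that distance, get a low CustomTimeDilation.
; Each is flagged and never restored here, and a debug string is printed.
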(event `self.ReceiveTick`
  (params (DeltaSeconds :type "Float (single-precision)"))
  ;[0 0.3765 1] Event tick check if bullet in range of player and slow it down
  (if (`Actor.HasAuthority` (`self.GetOwner`))
    _
    (else
      _))
  (`self.GetDistanceBetweenCharacters`)
  (`self.SlowDownBulletInRange`))

(fn `CheckBulletInRange`
  (params (BulletY :type "Float (double-precision)") (PlayerY :type "Float (double-precision)"))
  (returns (IsInRange :type Boolean))
  (bind _returnvalue (> (`local.BulletY`) (- (`local.PlayerY`) (* (`self.BulletDistancePercentageToCharacter`) (`KismetMathLibrary.Abs` (`self.DistanceBetweenPlayers`))))))
  (bind _returnvalue_2 (< (`local.BulletY`) (+ (`local.PlayerY`) (* (`self.BulletDistancePercentageToCharacter`) (`KismetMathLibrary.Abs` (`self.DistanceBetweenPlayers`))))))
  (if (> (`self.DistanceBetweenPlayers`) 0.0)
    (if _returnvalue_2
      (return _returnvalue_2))
    (elif _returnvalue
      (return _returnvalue))))

(fn `GetDistanceBetweenCharacters`
  (bind _returnvalue (`self.GetOwner`))
  (bind _outactors (`GameplayStatics.GetAllActorsOfClass` "/Game/Blueprints/Characters/FirstPersonCharacter.FirstPersonCharacter_C"))
  (for _array_element _outactors
    (if (not (== _returnvalue _array_element))
      (set `self.DistanceBetweenPlayers` (- (.y (`Actor.K2_GetActorLocation` _array_element)) (.y (`Actor.K2_GetActorLocation` _returnvalue)))))))

(fn `SlowDownBulletInRange`
  (locals (playerId :type Integer :default 0) (Bullet :type "/Game/Blueprints/Weapons/Projectiles/BaseProjectile Object Reference"))
  (bind _bullet (`local.Bullet`))
  (bind _y (.y (`Actor.K2_GetActorLocation` _bullet)))
  (bind _y_2 (.y (`Actor.K2_GetActorLocation` (`self.GetOwner`))))
  (bind _aspawn (cast `Pawn` (`self.GetOwner`)))
  (bind _asplayer_controller (cast `PlayerController` (`Pawn.GetController` _aspawn)))
  (set `local.playerId` (`PlayerState.PlayerId` (`Controller.PlayerState` _asplayer_controller)))
  (bind _outactors (`GameplayStatics.GetAllActorsOfClass` "/Game/Blueprints/Weapons/Projectiles/BaseProjectile.BaseProjectile_C"))
  (for _array_element _outactors
    (set `local.Bullet` _array_element)
    (if (`/Game/Blueprints/Weapons/Projectiles/BaseProjectile.b_SLowedDown` (`local.Bullet`))
      _
      (elif (not (== (`/Game/Blueprints/Weapons/Projectiles/BaseProjectile.PlayerNumber` _bullet) (`local.playerId`)))
        (bind _isinrange (`self.CheckBulletInRange` _y _y_2))
        (if _isinrange
          (`KismetSystemLibrary.PrintString` (`KismetStringLibrary.BuildString_Double` (`KismetStringLibrary.BuildString_Double` (`KismetStringLibrary.BuildString_Double` "" "Bullet y: " _y) " player y: " _y_2) " Distance between players: " (`self.DistanceBetweenPlayers`)) true true (struct :`G` 0.66 :`B` 1.0 :`A` 1.0) 999999.0)
          (set `Actor.CustomTimeDilation` 0.1 (`local.Bullet`))
          (set `/Game/Blueprints/Weapons/Projectiles/BaseProjectile.b_SLowedDown` true (`local.Bullet`)))))))