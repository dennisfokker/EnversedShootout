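; VR gun actor that fires player-tagged projectiles from its VRMarker, limited by overheating.
; ServerEvent_Fire adds heat before checking CanFire, so the shot that triggers lockout spawns no projectile.
; Tick cools the gun, re-enables firing only once heat reaches zero, and shows heat on a state-colored TextRender.
; For locally controlled instigators, Tick also destroys and respawns a laser-pointer beam emitter along the marker's forward vector.
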(event `self.ReceiveTick`
  (params (DeltaSeconds :type "Float (single-precision)"))
  ;[1 0.305 0] Event OnTick
  (`|ExecutionSequence`
    (:`then_0`
      (`self.UpdateCurrentOverheatingValue` DeltaSeconds))
    (:`then_1`
      (if (`Pawn.IsLocallyControlled` (`self.GetInstigator`))
        (`self.DrawLaserPointer`)))))

(event `ServerEvent_Fire`
  ;[1 1 0] Gun Logic
  ;;[1 1 1] Firing Event
  (`self.HandleOverheatingOnShot`)
  (if (`self.CanFire`)
    (bind _returnvalue (`|SpawnActorFromClass` "/Game/Blueprints/Weapons/Projectiles/FirstPersonProjectile.FirstPersonProjectile_C" (`KismetMathLibrary.MakeTransform` (.location (`SceneComponent.K2_GetComponentToWorld` (`self.VR_Marker`))) (.rotation (`SceneComponent.K2_GetComponentToWorld` (`self.VR_Marker`))) (0.2 0.2 0.2)) "AlwaysSpawn" "OverrideRootScale" null (`self.GetInstigator`))) ; Spawn projectile
    (set `/Game/Blueprints/Weapons/Projectiles/BaseProjectile.PlayerNumber` (`PlayerState.PlayerId` (`Controller.PlayerState` (`self.GetInstigatorController`))) _returnvalue)
    (`GameplayStatics.PlaySoundAtLocation` "/Game/Assets/Audio/FirstPersonTemplateWeaponFire02.FirstPersonTemplateWeaponFire02" (`self.K2_GetActorLocation`)) ; Play firing sound
  ))

(fn `CreateBeam`
  (params (StartLocation :type "Vector Structure") (EndLocation :type "Vector Structure"))
  (bind _laserbeam (`self.LaserBeam`))
  (`/Engine/EditorBlueprintResources/StandardMacros.IsValid` _laserbeam
    (:`Is Valid`
      (`ActorComponent.K2_DestroyComponent` _laserbeam))
    (:`Is Not Valid`
      _))
  (bind _returnvalue (`GameplayStatics.SpawnEmitterAtLocation` "/Game/Blueprints/Weapons/Projectiles/PS_LaserPointer.PS_LaserPointer" StartLocation))
  (bind _output_get (set `self.LaserBeam` _returnvalue))
  (`ParticleSystemComponent.SetBeamEndPoint` _output_get 0 EndLocation))

(fn `DrawLaserPointer`
  (bind _vr_marker (`self.VR_Marker`))
  (bind _output_get (set `self.BeamEndpoint` (+ (`SceneComponent.K2_GetComponentLocation` _vr_marker) (* (`SceneComponent.GetForwardVector` _vr_marker) 5000.0))))
  (set `self.BeamEndpoint` _output_get)
  (`self.CreateBeam` (`SceneComponent.K2_GetComponentLocation` (`self.VR_Marker`)) (`self.BeamEndpoint`)))

(fn `HandleOverheatingOnShot`
  (bind _returnvalue (+ (`self.CurrentOverheatingValue`) (`self.OverheatingValuePerShot`)))
  (if (`self.CanFire`)
    (set `self.CurrentOverheatingValue` _returnvalue)
    (if (not (< _returnvalue (`self.OverheatingTreshold`)))
      (set `self.CanFire` false))
    (return)))

(fn `RoundAndSetText`
  (params (OverheatingValue :type "Float (double-precision)"))
  (bind _textrender (`self.TextRender`))
  (`TextRenderComponent.K2_SetText` (`self.TextRender`) (`KismetTextLibrary.Conv_DoubleToText` (/ (`KismetMathLibrary.Conv_IntToDouble` (`KismetMathLibrary.Round` (* OverheatingValue 100.0))) 100.0) "HalfToEven"))
  (if (`self.CanFire`)
    (`TextRenderComponent.SetTextRenderColor` _textrender (`self.NormalColor`))
    (else
      (`TextRenderComponent.SetTextRenderColor` _textrender (`self.OverheatedColor`))))
  (return))

(fn `UpdateCurrentOverheatingValue`
  (params (DeltaSeconds :type "Float (double-precision)"))
  (bind _returnvalue (- (`self.CurrentOverheatingValue`) (* DeltaSeconds (`self.OverheatingSubractionValue`))))
  ;[1 1 1] Lower the current overheating value and set CanFire to true if it reaches 0.
  (if (< _returnvalue 0.0)
    (bind _output_get (set `self.CurrentOverheatingValue` 0.0))
    (set `self.CanFire` true)
    (`self.RoundAndSetText` _output_get)
    (else
      (bind _output_get_2 (set `self.CurrentOverheatingValue` _returnvalue))
      (`self.RoundAndSetText` _output_get_2)))
  (return))

(fn `UserConstructionScript`)