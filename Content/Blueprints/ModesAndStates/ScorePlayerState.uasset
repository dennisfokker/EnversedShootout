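; Player state that tracks a player's score and shows it on a score text actor in the level.
; Shortly after BeginPlay, the authority claims the first PlayerScoreTextObject numbered 0, stamps it with the PlayerId and resets its display.
; IncrementScore raises CurrentScore, whose RepNotify updates the claimed text.
; BeginPlay also starts 2D background music when the first player controller's pawn is locally controlled.
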(event `self.ReceiveBeginPlay`
  (`|ExecutionSequence`
    (:`then_0`
      (`KismetSystemLibrary.Delay` 0.05)
      (`/Engine/EditorBlueprintResources/ActorMacros.Switch Has Authority`
        (:`Authority`
          (bind _outactors (`GameplayStatics.GetAllActorsOfClass` "/Game/Blueprints/UI/PlayerScoreTextObject.PlayerScoreTextObject_C"))
          (for _array_element _outactors
            (if (== (`/Game/Blueprints/UI/PlayerScoreTextObject.PlayerNumber` _array_element) 0)
              (bind _output_get (set `self.PlayerScoreText` _array_element))
              (set `/Game/Blueprints/UI/PlayerScoreTextObject.PlayerNumber` (`self.PlayerId`) _array_element)
              (`/Game/Blueprints/UI/PlayerScoreTextObject.UpdateScore` _output_get 0)
              (break))))))
    (:`then_1`
      (if (`Pawn.IsLocallyControlled` (`Controller.K2_GetPawn` (`GameplayStatics.GetPlayerController` 0)))
        (`GameplayStatics.PlaySound2D` "/Game/Assets/Audio/BackgroundMusic.BackgroundMusic" 0.6)))))

(event `IncrementScore`
  (set `self.CurrentScore` (+ (`self.CurrentScore`) 1)))

(fn `OnRep_CurrentScore`
  (bind _playerscoretext (`self.PlayerScoreText`))
  (`/Engine/EditorBlueprintResources/StandardMacros.IsValid` _playerscoretext
    (:`Is Valid`
      (`/Game/Blueprints/UI/PlayerScoreTextObject.UpdateScore` _playerscoretext (`self.CurrentScore`)))))

(fn `UserConstructionScript`)